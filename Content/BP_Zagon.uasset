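; BP_Zagon is a sheep pen that counts delivered sheep and triggers the win screen.
; Any BP_Sheep overlapping ZagonArea is destroyed and tallied as rare or regular.
; Regular arrivals reveal Sheep1, or Sheep2 when their tally reaches SheepCount, both hidden at start.
; Reaching that target shows one of two end widgets, chosen by whether any rare sheep arrived, and switches input to game and UI.
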(event `self.ReceiveBeginPlay`
  (`SceneComponent.SetVisibility` (`self.Sheep1`) false false)
  (`SceneComponent.SetVisibility` (`self.Sheep2`) false false))

(event `self.ZagonArea.OnComponentBeginOverlap`
  (params (OverlappedComponent :type "PrimitiveComponent Object Reference") (OtherActor :type "Actor Object Reference") (OtherComp :type "PrimitiveComponent Object Reference") (OtherBodyIndex :type Integer) (bFromSweep :type Boolean) (SweepResult :type "HitResult Structure (by ref)"))
  (bind _asbp_sheep (cast `/Game/BP_Sheep` OtherActor))
  (if (`/Game/BP_Sheep.isRareSheep` _asbp_sheep)
    (`self.K2_DestroyActor` _asbp_sheep)
    (`/Engine/EditorBlueprintResources/StandardMacros.IncrementInt` (`self.sheepRareInZagon`))
    (else
      (`self.K2_DestroyActor` _asbp_sheep)
      (bind _result (`/Engine/EditorBlueprintResources/StandardMacros.IncrementInt` (`self.sheepInZagon`))
        (:`  `
          (if (== _result (`self.sheepCount`))
            (`SceneComponent.SetVisibility` (`self.Sheep2`) true false)
            (if (== (`self.sheepRareInZagon`) 0)
              (bind _returnvalue (`|CreateWidget` "/Game/WBP_Win.WBP_Win_C"))
              (`UserWidget.AddToViewport` _returnvalue 0)
              (`WidgetBlueprintLibrary.SetInputMode_GameAndUIEx` (`GameplayStatics.GetPlayerController` 0) _returnvalue)
              (else
                (bind _returnvalue_2 (`|CreateWidget` "/Game/WBP_Win1.WBP_Win1_C"))
                (`UserWidget.AddToViewport` _returnvalue_2 0)
                (`WidgetBlueprintLibrary.SetInputMode_GameAndUIEx` (`GameplayStatics.GetPlayerController` 0) _returnvalue_2)))
            (else
              (`SceneComponent.SetVisibility` (`self.Sheep1`) true false))))))))

(fn `UserConstructionScript`)
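; BP_Sheep is a sheep character that wanders randomly and bleats at random intervals, with randomized walk speed.
; Overlapping the player with its Sphere permanently switches Tick to AI MoveTo toward the player at a random per-sheep offset.
; Rare sheep get an alternate material and skip wandering.
; BurkArea tracks whether the player "dog" is near, but the bark-driven fear, herding and destroy logic is disconnected.
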(event `self.ReceiveBeginPlay`
  (bind _asbp_third_person_character (cast `/Game/ThirdPerson/Blueprints/BP_ThirdPersonCharacter` (`GameplayStatics.GetPlayerPawn` 0)))
  (set `self.Dog` _asbp_third_person_character)
  (`self.beee`)
  (set `CharacterMovementComponent.MaxWalkSpeed` (`KismetMathLibrary.RandomFloatInRange` 300.0 400.0) (`self.CharacterMovement`))
  (set `self.LocationOffset` (`KismetMathLibrary.MakeVector` (`KismetMathLibrary.RandomFloatInRange` 50.0 150.0) (`KismetMathLibrary.RandomFloatInRange` 50.0 150.0))))

(event `beee`
  (bind _returnvalue (`self.K2_GetActorLocation`))
  (`KismetSystemLibrary.Delay` (`KismetMathLibrary.RandomFloatInRange` 30.0 130.0))
  (switch `int` (`KismetMathLibrary.RandomIntegerInRange` 0 1)
    (:`0`
      (`GameplayStatics.PlaySoundAtLocation` "/Game/sound/ble1.ble1" _returnvalue (struct) 1.0 1.0 0.0 null null null null))
    (:`1`
      (`GameplayStatics.PlaySoundAtLocation` "/Game/sound/ble2.ble2" _returnvalue (struct) 1.0 1.0 0.0 null null null null)))
  (`self.beee`))

(event `self.Sphere.OnComponentBeginOverlap`
  (params (OverlappedComponent :type "PrimitiveComponent Object Reference") (OtherActor :type "Actor Object Reference") (OtherComp :type "PrimitiveComponent Object Reference") (OtherBodyIndex :type Integer) (bFromSweep :type Boolean) (SweepResult :type "HitResult Structure (by ref)"))
  (bind _asbp_third_person_character (cast `/Game/ThirdPerson/Blueprints/BP_ThirdPersonCharacter` OtherActor))
  (set `self.player` _asbp_third_person_character)
  (set `self.isGoToPlayer` true))

(event `self.ReceiveTick`
  (params (DeltaSeconds :type "Float (single-precision)"))
  (if (`self.isGoToPlayer`)
    (`|AIMoveTo` self (- (`self.K2_GetActorLocation` (`self.player`)) (`self.LocationOffset`)) null)
    (elif (and (`self.can go`) (not (`self.isRareSheep`)))
      (`self.go`))))

(event `self.Sphere.OnComponentEndOverlap`
  (params (OverlappedComponent :type "PrimitiveComponent Object Reference") (OtherActor :type "Actor Object Reference") (OtherComp :type "PrimitiveComponent Object Reference") (OtherBodyIndex :type Integer)))

(event `go`
  (set `self.can go` false)
  (`|AIMoveTo` self (+ (`self.K2_GetActorLocation`) (`KismetMathLibrary.MakeVector` (`KismetMathLibrary.RandomFloatInRange` -1200.0 1200.0) (`KismetMathLibrary.RandomFloatInRange` -1200.0 1200.0))) null 5.0 true
    (:`OnSuccess`
      (`KismetSystemLibrary.Delay` (`KismetMathLibrary.RandomFloatInRange` 3.0 7.0))
      (set `self.can go` true))))

(event `self.BurkArea.OnComponentBeginOverlap`
  (params (OverlappedComponent :type "PrimitiveComponent Object Reference") (OtherActor :type "Actor Object Reference") (OtherComp :type "PrimitiveComponent Object Reference") (OtherBodyIndex :type Integer) (bFromSweep :type Boolean) (SweepResult :type "HitResult Structure (by ref)"))
  (cast `/Game/ThirdPerson/Blueprints/BP_ThirdPersonCharacter` OtherActor)
  (set `self.DogInBurkArea` true))

(event `self.BurkArea.OnComponentEndOverlap`
  (params (OverlappedComponent :type "PrimitiveComponent Object Reference") (OtherActor :type "Actor Object Reference") (OtherComp :type "PrimitiveComponent Object Reference") (OtherBodyIndex :type Integer))
  (cast `/Game/ThirdPerson/Blueprints/BP_ThirdPersonCharacter` OtherActor)
  (set `self.DogInBurkArea` false))

(fn `UserConstructionScript`
  (if (`self.isRareSheep`)
    (`PrimitiveComponent.SetMaterial` (`self.Cube`) 0 "/Game/models/sheep2.sheep2")))
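; BP_WindArea is a wind zone that lets the third-person character smell while inside it, with a goal set at BeginPlay.
; Overlapping WindConnectionArea registers it as the character's current area and toggles the smell ability and UI; leaving keeps the registration.
; The goal is the sheep for the final point, otherwise the linked wind area.
; A Timeline for animating a direction Sign toward or from that goal is unwired, and ShowDir is empty.
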(event `self.ReceiveBeginPlay`
  (set `self.SheepLocation` (`self.K2_GetActorLocation` (`self.SheepPtr`)))
  (set `self.WindAreaLocation` (`self.K2_GetActorLocation` (`self.WindAreaPtr`)))
  (`SceneComponent.SetVisibility` (`self.Sign`) false false)
  (if (`self.IsFinalPoint`)
    (set `self.GoalLocation` (`self.SheepLocation`))
    (else
      (set `self.GoalLocation` (`self.WindAreaLocation`)))))

(event `self.WindConnectionArea.OnComponentBeginOverlap`
  (params (OverlappedComponent :type "PrimitiveComponent Object Reference") (OtherActor :type "Actor Object Reference") (OtherComp :type "PrimitiveComponent Object Reference") (OtherBodyIndex :type Integer) (bFromSweep :type Boolean) (SweepResult :type "HitResult Structure (by ref)"))
  (bind _asbp_third_person_character (cast `/Game/ThirdPerson/Blueprints/BP_ThirdPersonCharacter` OtherActor))
  (set `/Game/ThirdPerson/Blueprints/BP_ThirdPersonCharacter.CurrentWindArea` self _asbp_third_person_character)
  (set `/Game/ThirdPerson/Blueprints/BP_ThirdPersonCharacter.isCanSmell` true _asbp_third_person_character)
  (`Widget.SetVisibility` (`/Game/ThirdPerson/Blueprints/BP_ThirdPersonCharacter.SmellInterf` _asbp_third_person_character) "Visible"))

(event `self.WindConnectionArea.OnComponentEndOverlap`
  (params (OverlappedComponent :type "PrimitiveComponent Object Reference") (OtherActor :type "Actor Object Reference") (OtherComp :type "PrimitiveComponent Object Reference") (OtherBodyIndex :type Integer))
  (bind _asbp_third_person_character (cast `/Game/ThirdPerson/Blueprints/BP_ThirdPersonCharacter` OtherActor))
  (set `/Game/ThirdPerson/Blueprints/BP_ThirdPersonCharacter.CurrentWindArea` self _asbp_third_person_character)
  (set `/Game/ThirdPerson/Blueprints/BP_ThirdPersonCharacter.isCanSmell` false _asbp_third_person_character)
  (`Widget.SetVisibility` (`/Game/ThirdPerson/Blueprints/BP_ThirdPersonCharacter.SmellInterf` _asbp_third_person_character) "Hidden"))

(fn `ShowDir`)

(fn `UserConstructionScript`)